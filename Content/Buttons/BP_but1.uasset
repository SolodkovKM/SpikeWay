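; BP_but1 is a one-shot push button that sends a referenced actor, apparently a turtle, along a spline.
; The box trigger toggles input and a press prompt.
; A press, gated by IsTurttleComing, plays an explosion, then chained timelines scale the actor at the first spline and move it along another.
; On arrival a second explosion plays, the Tumb and Button components are destroyed and the prompt stays hidden.
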(event OnComponentBeginOverlap(Box)
  (params (OverlappedComponent :type Primitive%20Component%20Object%20Reference) (OtherActor :type Actor%20Object%20Reference) (OtherComp :type Primitive%20Component%20Object%20Reference) (OtherBodyIndex :type Integer) (bFromSweep :type Boolean) (SweepResult :type Hit%20Result%20Structure%20%28by%20ref%29))
  (Input|EnableInput (Game|GetPlayerController 0))
  (if (not (Variables|Default|GetUnVisibleText))
    (Rendering|SetVisibility (Variables|Default|Getbuttonpres) true false)))

(event OnComponentEndOverlap(Box)
  (params (OverlappedComponent :type Primitive%20Component%20Object%20Reference) (OtherActor :type Actor%20Object%20Reference) (OtherComp :type Primitive%20Component%20Object%20Reference) (OtherBodyIndex :type Integer))
  (Input|DisableInput (Game|GetPlayerController 0))
  (Rendering|SetVisibility (Variables|Default|Getbuttonpres) false false))

(event Input|ActionEvents|InputActionbutton_press
  (params (Key :type Key%20Structure :default "None"))
  (:Pressed
    (if (Variables|Default|GetIsTurttleComing)
      (Audio|PlaySoundatLocation "/Game/StarterContent/Audio/Explosion01.Explosion01" "0, 0, 0" "0, 0, 0" 1.0 1.0 0.0 0 0 0 0)
      (Effects|SpawnEmitteratLocation "/Game/StarterContent/Particles/P_Explosion.P_Explosion" (Spline|GetLocationatTime (Variables|Default|GetSpline1) 0.0 "World" false))
      (bind _newtrack_0 (Timeline|Timeline_1 Play)
        (:Update
          (Transformation|SetActorTransform (Variables|Default|GetActor) (Math|Transform|MakeTransform (Spline|GetLocationatSplinePoint (Variables|Default|GetSpline1) 0 "World") "0,-90.000000, 0" (Math|Vector|MakeVector _newtrack_0 _newtrack_0 _newtrack_0))))
        (:Finished
          (bind _newtrack_1 (Timeline|Timeline_0 Play)
            (:Update
              (Transformation|SetActorTransform (Variables|Default|GetActor) (Math|Transform|MakeTransform (Spline|GetLocationatTime (Variables|Default|GetSpline) _newtrack_1 "World" false) "0,-90.000000, 0" "0.400000,0.400000,0.400000"))
              (Variables|Default|SetIsTurttleComing (not (> _newtrack_1 0.0))))
            (:Finished
              (Audio|PlaySoundatLocation "/Game/StarterContent/Audio/Explosion02.Explosion02" "0, 0, 0" "0, 0, 0" 1.0 1.0 0.0 0 0 0 0)
              (Effects|SpawnEmitteratLocation "/Game/StarterContent/Particles/P_Explosion.P_Explosion" (Spline|GetLocationatTime (Variables|Default|GetSpline2) 0.0 "World" false))
              (Components|DestroyComponent (Variables|Default|GetTumb))
              (Rendering|SetVisibility (Variables|Default|Getbuttonpres) false false)
              (Variables|Default|SetUnVisibleText true))))))))

(fn ConstructionScript)